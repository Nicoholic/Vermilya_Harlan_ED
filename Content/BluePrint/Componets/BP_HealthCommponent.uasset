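; Health component that tracks current health for its owning actor and reports hurt and death.
; On BeginPlay it fills health to maximum and binds to the owner's OnTakeAnyDamage event.
; Each hit subtracts clamped damage, then calls OnHurt with the health fraction, or unbinds from damage and calls OnDeath at zero.
; It also prints current health after every hit.
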(event Custom|HandleDamage
  (params (DamagedActor :type Actor%20Object%20Reference) (Damage :type Float%20%28single-precision%29) (DamageType :type Damage%20Type%20Object%20Reference) (InstigatedBy :type Controller%20Object%20Reference) (DamageCauser :type Actor%20Object%20Reference))
  (bind _output_get (Variables|Default|SetCurrent%20Health (Math|Float|Clamp(Float) (- (Variables|Default|GetCurrent%20Health) Damage) 0.0 (Variables|Default|GetMax%20Health))))
  (if (> _output_get 0.0)
    (Default|CallOnHurt (/ (Variables|Default|GetCurrent%20Health) (Variables|Default|GetMax%20Health)))
    (else
      (EventDispatchers|UnbindEventfromOnTakeAnyDamage (Components|GetOwner) (EventDispatchers|CreateEvent :!event Custom|HandleDamage))
      (Default|CallOnDeath 0.0)))
  (Development|PrintString (Utilities|String|ToString(Float) _output_get)))

(event EventBeginPlay
  (EventDispatchers|BindEventtoOnTakeAnyDamage (Components|GetOwner) (EventDispatchers|CreateEvent :!event Custom|HandleDamage))
  (Variables|Default|SetCurrent%20Health (Variables|Default|GetMax%20Health)))