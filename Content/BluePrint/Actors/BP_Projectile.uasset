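; Projectile actor that damages whatever its collision sphere overlaps, then destroys itself.
; The construction script scales the sphere and binds its begin-overlap delegate.
; BeginPlay calls the parent, starts a one-shot timer using DestoryTimer, and caches the owner as damage instigator, printing a warning unless that owner is a Controller.
; The sphere's hit event only prints a debug string.
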(event OnComponentHit(SphereCollision)
  (params (HitComponent :type Primitive%20Component%20Object%20Reference) (OtherActor :type Actor%20Object%20Reference) (OtherComp :type Primitive%20Component%20Object%20Reference) (NormalImpulse :type Vector :default "0, 0, 0") (Hit :type Hit%20Result%20Structure%20%28by%20ref%29))
  ;[1 1 1] in code already
  (Development|PrintString "Hello"))

(event Custom|HandleOverLap
  (params (OverlappedComponent :type Primitive%20Component%20Object%20Reference) (OtherActor :type Actor%20Object%20Reference) (OtherComp :type Primitive%20Component%20Object%20Reference) (OtherBodyIndex :type Integer) (bFromSweep :type Boolean) (SweepResult :type Hit%20Result%20Structure%20%28by%20ref%29))
  (Game|Damage|ApplyDamage OtherActor (Variables|Default|GetDamage) (Variables|Default|GetController) self)
  (Actor|DestroyActor))

(event EventBeginPlay
  ;[1 1 1] this is the equilevent to super
  (|CallParentFunction)
  (Utilities|Time|SetTimerbyEvent (EventDispatchers|CreateEvent :!event K2DestroyActor) (Variables|Default|GetDestoryTimer))
  (bind _ascontroller (Utilities|Casting|CastToController (Components|GetOwner))
    (:then
      (Variables|Default|SetController _ascontroller))
    (:CastFailed
      (Development|PrintString "we need an owner "))))

(event Collision|EventActorBeginOverlap
  (params (OtherActor :type Actor%20Object%20Reference)))

(fn ConstructionScript
  (bind _spherecollision (Variables|Default|GetSphereCollision))
  (Collision|BindEventtoOnComponentBeginOverlap _spherecollision (EventDispatchers|CreateEvent :!event Custom|HandleOverLap))
  (Transformation|SetWorldScale3D _spherecollision (Variables|Default|GetScale)))