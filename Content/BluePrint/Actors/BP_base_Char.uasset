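; BP_base_Char is a base character Blueprint that sets up a weapon, health events and animation links on BeginPlay.
; It spawns WeaponClass through a child actor component, then caches it as a BP_Rifle alongside the mesh's ABP_CharacterAnimation.
; It binds to rifle fire and reload start, health hurt and death, and animation reload notifications.
; If either cast fails, it prints an error and destroys itself.
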(event EventBeginPlay
  (bind _childactorcomponent (Variables|Default|GetChildActorComponent))
  (|CallParentFunction)
  (ChildActorComponent|SetChildActorClass _childactorcomponent (Variables|Default|GetWeaponClass))
  (bind _asbp_rifle (Utilities|Casting|CastToBP_Rifle (Variables|/Script/Engine.ChildActorComponent|GetChildActor _childactorcomponent))
    (:then
      (Variables|Default|SetWeapon _asbp_rifle)
      (bind _asabp_character_animation (Utilities|Casting|CastToABP_CharacterAnimation (Components|SkeletalMesh|GetAnimInstance (Variables|Character|GetMesh)))
        (:then
          (Variables|Default|Set%20AnimationBP _asabp_character_animation)
          (EventDispatchers|BindEventtoOnRifleFire (Variables|Default|GetWeapon) (EventDispatchers|CreateEvent (Variables|Default|Get%20AnimationBP) :!event AttackAnim))
          (EventDispatchers|BindEventtoOnHurt (Variables|Default|GetHealthCommponent) (EventDispatchers|CreateEvent (Variables|Default|Get%20AnimationBP) :!event HurtAnimation))
          (EventDispatchers|BindEventtoOnDeath (Variables|Default|GetHealthCommponent) (EventDispatchers|CreateEvent (Variables|Default|Get%20AnimationBP) :!event DeadAnimation))
          (EventDispatchers|BindEventtoOnReloadStart (Variables|Default|GetWeapon) (EventDispatchers|CreateEvent (Variables|Default|Get%20AnimationBP) :!event ReloadAnimation))
          (EventDispatchers|BindEventtoOnReloadEnded (Variables|Default|Get%20AnimationBP) (EventDispatchers|CreateEvent (Variables|Default|GetWeapon) :!event ActionStop))
          (EventDispatchers|BindEventtoOnReloadNow (Variables|Default|Get%20AnimationBP) (EventDispatchers|CreateEvent (Variables|Default|GetWeapon) :!event ReloadAmmo)))
        (:CastFailed
          (Development|PrintString "we need the correct animiation for the char")
          (Actor|DestroyActor))))
    (:CastFailed
      (Development|PrintString "We need a weapon for the characters")
      (Actor|DestroyActor))))

(event Collision|EventActorBeginOverlap
  (params (OtherActor :type Actor%20Object%20Reference)))

(event EventTick
  (params (DeltaSeconds :type Float%20%28single-precision%29)))

(fn ConstructionScript)