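; Player pawn Blueprint that handles movement, camera look, weapon input and HUD setup.
; On BeginPlay it creates the HUD, binds health hurt/death and weapon ammo-change events, then reloads the weapon; without a PlayerController it destroys itself.
; Movement follows control yaw only, while attack and reload inputs delegate to the Weapon.
; HandleDeath disables player input.
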(event EventBeginPlay
  (bind _healthcommponent (Variables|Default|GetHealthCommponent))
  (bind _weapon (Variables|Default|GetWeapon))
  (|CallParentFunction)
  (bind _asplayer_controller (Utilities|Casting|CastToPlayerController (Pawn|GetController))
    (:then
      (bind _output_get (Variables|Default|SetPlayer%20Controller _asplayer_controller))
      (bind _returnvalue (UserInterface|CreateWidget (Variables|Default|GetHudClass) _output_get))
      (UserInterface|Viewport|AddtoViewport _returnvalue 0)
      (EventDispatchers|BindEventtoOnHurt _healthcommponent (EventDispatchers|CreateEvent _returnvalue :!event SetHealth))
      (EventDispatchers|BindEventtoOnDeath _healthcommponent (EventDispatchers|CreateEvent _returnvalue :!event SetHealth))
      (EventDispatchers|BindEventtoOnAmmoChange _weapon (EventDispatchers|CreateEvent _returnvalue :!event SetAmmo))
      (Default|ReloadAmmo _weapon))
    (:CastFailed
      (Development|PrintString "We need a controller to make the HUD")
      (Actor|DestroyActor))))

(event Collision|EventActorBeginOverlap
  (params (OtherActor :type Actor%20Object%20Reference))
  (|CallParentFunction OtherActor) ; This node is disabled and will not be called.\nDrag off pins to build functionality.
)

(event EventTick
  (params (DeltaSeconds :type Float%20%28single-precision%29))
  (|CallParentFunction DeltaSeconds) ; This node is disabled and will not be called.\nDrag off pins to build functionality.
)

(event EventHandleDeath
  (params (Ratio :type Float%20%28single-precision%29))
  (Input|DisableInput (Variables|Default|GetPlayer%20Controller)))

(event Input|ActionEvents|InputActionAttackInput
  (params (Key :type Key%20Structure :default "None"))
  (:Pressed
    (Default|Attack (Variables|Default|GetWeapon))))

(event Input|ActionEvents|InputActionReloading
  (params (Key :type Key%20Structure :default "None"))
  (:Pressed
    (Default|RequestReload (Variables|Default|GetWeapon))))

(event Input|AxisEvents|InputAxisTurnRight
  (params (AxisValue :type Float%20%28single-precision%29))
  ;[1 1 1] In code
  (Pawn|Input|AddControllerYawInput AxisValue))

(event Input|AxisEvents|InputAxisLookUp
  (params (AxisValue :type Float%20%28single-precision%29))
  (Pawn|Input|AddControllerPitchInput AxisValue))

(event Input|AxisEvents|InputAxisMoveForward
  (params (AxisValue :type Float%20%28single-precision%29))
  (Pawn|Input|AddMovementInput (Math|Vector|GetForwardVector (Math|Rotator|MakeRotator 0.0 0.0 (.yaw (Pawn|GetControlRotation :!class /Script/Engine.Pawn)))) AxisValue false))

(event Input|AxisEvents|InputAxisMoveRight
  (params (AxisValue :type Float%20%28single-precision%29))
  (Pawn|Input|AddMovementInput (Math|Vector|GetRightVector (Math|Rotator|MakeRotator 0.0 0.0 (.yaw (Pawn|GetControlRotation :!class /Script/Engine.Pawn)))) AxisValue false))

(fn ConstructionScript
  (|CallParentFunction))