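; BP_Agent is an AI-controlled agent Blueprint that carries a weapon and reports its ammo to its AI.
; On BeginPlay it tints the mesh materials with its color, stops the weapon action, binds an ammo-change callback and reloads.
; Tick calls the weapon's attack every frame, while EnemyAttack and EnemyReload events forward attack and reload requests to the weapon.
; UpdateAmmo writes the current ammo count to the AI controller's Blackboard.
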(event EventBeginPlay
  (bind _weapon (Variables|Default|GetWeapon))
  (|CallParentFunction)
  (Rendering|Material|SetVectorParameterValueonMaterials (Variables|Character|GetMesh) "BodyColor" (Math|Conversions|ToVector(LinearColor) (Variables|Default|GetColor)))
  (Default|ActionStop _weapon)
  (EventDispatchers|BindEventtoOnAmmoChange _weapon (EventDispatchers|CreateEvent :!event UpdateAmmo))
  (Default|ReloadAmmo _weapon))

(event EventEnemyAttack
  (Default|Attack (Variables|Default|GetWeapon)))

(event EventTick
  (params (DeltaSeconds :type Float%20%28single-precision%29))
  (Default|Attack (Variables|Default|GetWeapon)))

(event EventEnemyReload
  (Default|RequestReload (Variables|Default|GetWeapon)))

(fn ConstructionScript
  (|CallParentFunction))

(fn UpdateAmmo
  (params (Current :type Float%20%28single-precision%29) (Max :type Float%20%28single-precision%29))
  (AI|Components|Blackboard|SetValueasFloat (AI|GetBlackboard (AI|GetAIController self)) (Variables|Default|GetAmmo%20Name) Current))