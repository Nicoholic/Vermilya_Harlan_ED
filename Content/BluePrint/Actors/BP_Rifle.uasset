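; BP_Rifle is a rifle actor that must be a child actor of a pawn, spawning projectiles and tracking ammo.
; Attack checks ammo, owner alive state and a busy flag, then fires from the muzzle socket, starts a shot timer and consumes ammo.
; Aim points toward the first HUD widget's Endpoint if that HUD's player owns the rifle, otherwise along base aim rotation.
; Fire, reload-start and ammo changes are broadcast through dispatchers.
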(event Custom|ActionStop
  (Variables|Default|SetActionHappening false))

(event Custom|OwnerDied
  (Variables|Default|SetAlive false))

(event Custom|ReloadAmmo
  (bind _max (Variables|Default|GetMax))
  (bind _output_get (Variables|Default|SetCurrent _max))
  (Default|CallOnAmmoChange _output_get _max))

(event Custom|UseAmmo
  (bind _output_get (Variables|Default|SetCurrent (Math|Float|Max(Float) (- (Variables|Default|GetCurrent) 1.0) 0.0)))
  (Default|CallOnAmmoChange _output_get (Variables|Default|GetMax)))

(event Custom|RequestReload
  (if (not (Variables|Default|GetActionHappening))
    (Variables|Default|SetActionHappening true)
    (Default|CallOnReloadStart)))

(event EventBeginPlay
  (bind _aspawn (Utilities|Casting|CastToPawn (Actor|GetParentActor))
    (:then
      (Variables|Default|SetParentPawn _aspawn)
      (CallFunction|ReloadAmmo))
    (:CastFailed
      (Development|PrintString "Must be owned by a pawn")
      (Actor|DestroyActor))))

(fn ConstructionScript)

(fn Attack
  (bind _parentpawn (Variables|Default|GetParentPawn))
  (if (CallFunction|CanShoot)
    (Game|SpawnActorfromClass (Variables|Default|GetProjectileClass) (Math|Transform|MakeTransform (CallFunction|GetShotLocation) (CallFunction|DoNotExporttoCode) "1,1,1") "Undefined" (Pawn|GetController _parentpawn) _parentpawn)
    (Variables|Default|SetActionHappening true)
    (Utilities|Time|SetTimerbyEvent (EventDispatchers|CreateEvent :!event Custom|ActionStop) (Variables|Default|GetShotTime))
    (Default|CallOnRifleFire)
    (CallFunction|UseAmmo)))

(fn CanShoot
  (return (Math|Boolean|ANDBoolean (not (Variables|Default|GetActionHappening)) (Variables|Default|GetAlive) (> (Variables|Default|GetCurrent) 0.0))))

(fn DoNotExporttoCode
  (bind _foundwidgets (Widget|GetAllWidgetsOfClass "/Game/Both/WBP_HUD.WBP_HUD_C" false))
  (if (== (Class|UserWidget|GetOwningPlayerPawn (Utilities|Array|Get(acopy) _foundwidgets)) (Variables|Default|GetParentPawn))
    (return (Math|Rotator|MakeRotfromX (- (Variables|/Script/Vermilya_Harlan_ED.GameHUD|GetEndpoint (Utilities|Array|Get(acopy) _foundwidgets)) (CallFunction|GetShotLocation))))
    (else
      (return (Pawn|GetBaseAimRotation (Variables|Default|GetParentPawn))))))

(fn GetShotLocation
  (return (Transformation|GetSocketLocation (Variables|Default|GetSkeletalMesh) "MuzzleFlashSocket")))